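; StaticLightBP is a furniture light that flickers two point lights continuously during play.
; From BeginPlay, a chain of Delay nodes toggles both lights together between full intensity and off in two quick blinks, then holds them lit briefly.
; The chain wires back to its start, repeating the fixed pattern indefinitely without Tick, timelines or randomness.
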(event `self.ReceiveBeginPlay`
  (`LightComponent.SetIntensity` (`self.PointLight`) 10000.0 :!label _label)
  (`LightComponent.SetIntensity` (`self.PointLight1`) 10000.0)
  (`KismetSystemLibrary.Delay` 0.1)
  (`LightComponent.SetIntensity` (`self.PointLight`) 0.0)
  (`LightComponent.SetIntensity` (`self.PointLight1`) 0.0)
  (`KismetSystemLibrary.Delay` 0.1)
  (`LightComponent.SetIntensity` (`self.PointLight`) 10000.0)
  (`LightComponent.SetIntensity` (`self.PointLight1`) 10000.0)
  (`KismetSystemLibrary.Delay` 0.1)
  (`LightComponent.SetIntensity` (`self.PointLight`) 0.0)
  (`LightComponent.SetIntensity` (`self.PointLight1`) 0.0)
  (`KismetSystemLibrary.Delay` 0.1)
  (`LightComponent.SetIntensity` (`self.PointLight`) 10000.0)
  (`LightComponent.SetIntensity` (`self.PointLight1`) 10000.0)
  (`KismetSystemLibrary.Delay` 0.75)
  (goto _label))

(fn `UserConstructionScript`)