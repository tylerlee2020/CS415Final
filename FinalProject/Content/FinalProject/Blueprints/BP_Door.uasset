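; BP_Door is a hinged door actor that can be locked behind a colored keycard.
; OpenDoor prints a message naming the required keycard color while Locked, otherwise a FlipFlop alternates between opening and closing on each call.
; A timeline drives the door's relative yaw through a Lerp to a quarter turn and reverses to close it.
; The unlockDoor event clears the Locked flag.
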(event `OpenDoor`
  (if (`self.Locked`)
    (`KismetSystemLibrary.PrintString` (`KismetStringLibrary.Concat_StrStr` "Door is locked look for the " (`self.Color`) " Keycard"))
    (else
      (`/Engine/EditorBlueprintResources/StandardMacros.FlipFlop`
        (:`A`
          (bind (_direction _doorrotate) (`Timeline|openDoorTimeline` :!via `PlayFromStart` :!label _label)
            (:`Update`
              (`SceneComponent.K2_SetRelativeRotation` (`self.Door`) (`KismetMathLibrary.MakeRotator` 0.0 0.0 (`KismetMathLibrary.Lerp` 0.0 90.0 _doorrotate)) false false))))
        (:`B`
          (goto _label :!via `Reverse`))))))

(event `unlockDoor`
  (params (NewParam :type Integer))
  (set `self.Locked` false))

(fn `UserConstructionScript`)