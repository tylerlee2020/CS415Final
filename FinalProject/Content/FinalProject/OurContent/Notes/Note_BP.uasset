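; Note_BP is a readable note the player picks up and puts down with the E key, using input enabled at BeginPlay.
; E line-traces from the first-person camera for WorldDynamic objects and checks for a hit static mesh component named "Note".
; A match hides that component's owning actor and shows a NoteWidget_BP on screen.
; Pressing E again removes the widget and unhides the actor.
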(event `Key|E`
  (params (Key :type "Key Structure"))
  (:`Pressed`
    (if (`self.HoldingNote`)
      (`Widget.RemoveFromParent` (`self.NoteRef`))
      (`self.SetActorHiddenInGame` (`ActorComponent.GetOwner` (`self.Static Mesh Ref`)) false)
      (set `self.HoldingNote` false)
      (else
        (bind _aszachs_first_person_character (cast `/Game/FinalProject/Blueprints/ZachsFirstPersonCharacter` (`GameplayStatics.GetPlayerCharacter` 0)))
        (bind _firstpersoncamera (`/Game/FinalProject/Blueprints/ZachsFirstPersonCharacter.FirstPersonCamera` _aszachs_first_person_character))
        (bind _returnvalue (`SceneComponent.K2_GetComponentLocation` _firstpersoncamera))
        (bind (_outhit _returnvalue_2) (`KismetSystemLibrary.LineTraceSingleForObjects` :`Start` _returnvalue :`End` (+ _returnvalue (* (`SceneComponent.GetForwardVector` _firstpersoncamera) (500.0 500.0 500.0))) :`ObjectTypes` (`|MakeArray` "ObjectTypeQuery2" :!type "EObjectTypeQuery Enum") :`bTraceComplex` true :`bIgnoreSelf` false))
        (if _returnvalue_2
          (bind _asstatic_mesh_component (cast `StaticMeshComponent` (`.HitComponent` (`GameplayStatics.BreakHitResult` _outhit))))
          (bind _output_get (set `self.Static Mesh Ref` _asstatic_mesh_component))
          (bind _returnvalue_3 (`KismetSystemLibrary.GetObjectName` _output_get))
          (`KismetSystemLibrary.PrintText` (`KismetTextLibrary.Conv_StringToText` _returnvalue_3))
          (if (`KismetStringLibrary.EqualEqual_StrStr` _returnvalue_3 "Note")
            (set `self.HoldingNote` true)
            (`self.SetActorHiddenInGame` (`ActorComponent.GetOwner` _output_get) true)
            (bind _returnvalue_4 (`|CreateWidget` "/Game/FinalProject/OurContent/Notes/NoteWidget_BP.NoteWidget_BP_C"))
            (bind _output_get_2 (set `self.NoteRef` _returnvalue_4))
            (`UserWidget.AddToViewport` _output_get_2 0)))))))

(event `self.ReceiveBeginPlay`
  (`self.EnableInput` (`GameplayStatics.GetPlayerController` 0)))

(fn `UserConstructionScript`)