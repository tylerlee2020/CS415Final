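; Electric box actor that launches the wire-connecting minigame when the first-person character walks into its collision box.
; An overlap on an unfinished box pauses the game, shows the WWireBoard widget at a fixed size and position, and enables the mouse cursor.
; A Solving flag, set before the character cast, blocks repeat triggers.
; CloseBox calls BoxClose, which snaps the power box mesh to a closed rotation and location.
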(event `self.CollisionBox.OnComponentBeginOverlap`
  (params (OverlappedComponent :type "PrimitiveComponent Object Reference") (OtherActor :type "Actor Object Reference") (OtherComp :type "PrimitiveComponent Object Reference") (OtherBodyIndex :type Integer) (bFromSweep :type Boolean) (SweepResult :type "HitResult Structure (by ref)"))
  (if (not (`self.Solving`))
    (set `self.Solving` true)
    (cast `/Game/FinalProject/Blueprints/ZachsFirstPersonCharacter` OtherActor)
    (if (not (`self.Complete`))
      (`GameplayStatics.SetGamePaused` true)
      (bind _returnvalue (`|CreateWidget` "/Game/FinalProject/Minigames/ConnectWire/wWireBoard.wWireBoard_C"))
      (`UserWidget.AddToViewport` _returnvalue 0)
      (`KismetSystemLibrary.PrintString` "added")
      (`UserWidget.SetDesiredSizeInViewport` _returnvalue (1024.0 768.0))
      (`UserWidget.SetPositionInViewport` _returnvalue (420.0 75.0) true)
      (set `PlayerController.bShowMouseCursor` true (`GameplayStatics.GetPlayerController` 0)) ; Make sure that the player can see the mouse so that they know what they're clicking.
    )))

(event `BoxClose`
  (bind _cube_003_power_box_0 (`self.Cube_003_Power_box_0`))
  (`SceneComponent.K2_SetRelativeRotation` _cube_003_power_box_0 (`KismetMathLibrary.MakeRotator` 0.0 0.0 -90.0) false false)
  (`SceneComponent.K2_SetRelativeLocation` _cube_003_power_box_0 (-80.0 -20.0 0.0) false false))

(fn `CloseBox`
  (`self.BoxClose`)
  (return))

(fn `UserConstructionScript`)