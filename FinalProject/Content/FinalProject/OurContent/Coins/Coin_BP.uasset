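; Coin pickup actor that adds to the player's wallet when collected.
; Overlap with the PickUpRadius component casts the overlapping actor's instigator to ZachsFirstPersonCharacter.
; On success it plays a coin sound at the mesh location, increments Wallet, destroys itself, and prints the new total to screen.
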(event `self.PickUpRadius.OnComponentBeginOverlap`
  (params (OverlappedComponent :type "PrimitiveComponent Object Reference") (OtherActor :type "Actor Object Reference") (OtherComp :type "PrimitiveComponent Object Reference") (OtherBodyIndex :type Integer) (bFromSweep :type Boolean) (SweepResult :type "HitResult Structure (by ref)"))
  (bind _aszachs_first_person_character (cast `/Game/FinalProject/Blueprints/ZachsFirstPersonCharacter` (`self.GetInstigator` OtherActor)))
  (`GameplayStatics.PlaySoundAtLocation` "/Game/FinalProject/OurContent/SoundEffects/Coin.Coin" (`SceneComponent.K2_GetComponentLocation` (`self.CoinMesh`)) (struct) 1.0 1.0 0.0 null null null null)
  (`/Engine/EditorBlueprintResources/StandardMacros.IncrementInt` (`/Game/FinalProject/Blueprints/ZachsFirstPersonCharacter.Wallet` _aszachs_first_person_character)
    (:`  `
      (`self.K2_DestroyActor`)
      (`KismetSystemLibrary.PrintString` (`KismetStringLibrary.Conv_IntToString` (`/Game/FinalProject/Blueprints/ZachsFirstPersonCharacter.Wallet` _aszachs_first_person_character))))))

(fn `UserConstructionScript`)