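; LightBP is a furniture light with two point lights that can be switched on and off.
; The ToggleLights event flips the IsOn flag, applies it to both lights' visibility and sets their color from the LightColor variable.
; The construction script applies IsOn to the lights' visibility as the initial state, without setting the color.
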(event `/Game/FinalProject/OurContent/FurnitureContent/Light/Lights_Int.Toggle Lights`
  (bind _output_get (set `self.is on?` (not (`self.is on?`))))
  (`SceneComponent.SetVisibility` (`self.PointLight`) _output_get false)
  (`SceneComponent.SetVisibility` (`self.PointLight1`) _output_get false)
  (`LightComponent.SetLightColor` (`self.PointLight`) (`self.Light Color`) true)
  (`LightComponent.SetLightColor` (`self.PointLight1`) (`self.Light Color`) true))

(fn `UserConstructionScript`
  (`SceneComponent.SetVisibility` (`self.PointLight`) (`self.is on?`) false)
  (`SceneComponent.SetVisibility` (`self.PointLight1`) (`self.is on?`) false))