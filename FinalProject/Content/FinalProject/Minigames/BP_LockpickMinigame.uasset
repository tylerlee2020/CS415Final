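; Lockpicking minigame actor that shows a lockpick widget and hands player input from the character to itself.
; A SceneCapture2D renders only this actor's own components.
; Left and Right keys open gates that Tick passes through, setting RightPickScene to fixed Speed-based relative rotations rather than accumulating.
; Matching A and D gates also target RightPickScene, but their Enter sequence is unconnected, so they never rotate it.
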(event `self.ReceiveBeginPlay`
  (bind _returnvalue (`GameplayStatics.GetPlayerController` 0))
  (bind _returnvalue_2 (`|CreateWidget` "/Game/FinalProject/Minigames/LockpickWidget.LockpickWidget_C"))
  (`UserWidget.AddToViewport` _returnvalue_2 0)
  (`SceneCaptureComponent.ShowOnlyActorComponents` (`self.SceneCaptureComponent2D`) self false) ; Make it so that only the lockpick elements themselves are shown.
  (`self.DisableInput` (`GameplayStatics.GetPlayerCharacter` 0) _returnvalue) ; Make sure the player can't do anything while playing the minigame.
  (`self.EnableInput` _returnvalue) ; Enable input for the minigame itself.
)

(event `Key|Left`
  (params (Key :type "Key Structure"))
  (:`Pressed`
    (goto _label :!via `Open`))
  (:`Released`
    (goto _label :!via `Close`)))

(event `self.ReceiveTick`
  (params (DeltaSeconds :type "Float (single-precision)"))
  (bind _speed (`self.Speed`))
  (bind _rightpickscene (`self.RightPickScene`))
  (`|ExecutionSequence`
    (:`then_0`
      (`/Engine/EditorBlueprintResources/StandardMacros.Gate` true :!label _label
        (:`Exit`
          (`SceneComponent.K2_SetRelativeRotation` _rightpickscene (`KismetMathLibrary.MakeRotator` 0.0 0.0 (* _speed -1.0)) false false))))
    (:`then_1`
      (`/Engine/EditorBlueprintResources/StandardMacros.Gate` true :!label _label_2
        (:`Exit`
          (`SceneComponent.K2_SetRelativeRotation` _rightpickscene (`KismetMathLibrary.MakeRotator` _speed) false false))))))

(event `Key|Right`
  (params (Key :type "Key Structure"))
  (:`Pressed`
    (goto _label_2 :!via `Open`))
  (:`Released`
    (goto _label_2 :!via `Close`)))

(event `Key|A`
  (params (Key :type "Key Structure"))
  (:`Pressed`
    (`/Engine/EditorBlueprintResources/StandardMacros.Gate` true :!via `Open` :!label _label_3
      (:`Exit`
        (`SceneComponent.K2_SetRelativeRotation` (`self.RightPickScene`) (`KismetMathLibrary.MakeRotator` 0.0 0.0 (* (`self.Speed`) -1.0)) false false))))
  (:`Released`
    (goto _label_3 :!via `Close`)))

(event `Key|D`
  (params (Key :type "Key Structure"))
  (:`Pressed`
    (`/Engine/EditorBlueprintResources/StandardMacros.Gate` true :!via `Open` :!label _label_4
      (:`Exit`
        (`SceneComponent.K2_SetRelativeRotation` (`self.RightPickScene`) (`KismetMathLibrary.MakeRotator` (* (`self.Speed`) -1.0)) false false))))
  (:`Released`
    (goto _label_4 :!via `Close`)))

(fn `UserConstructionScript`)