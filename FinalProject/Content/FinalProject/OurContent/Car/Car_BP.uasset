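; Car actor that serves as a scripted boss finisher, ending in the spawn of the winning acorn.
; On BeginPlay it finds the BossPinto, and a timeline slides the car along negative world X from its start position.
; When the timeline finishes, it spawns a huge explosion, destroys the boss and itself, then spawns BP_Winning_Acorn using its own location.
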(event `self.ReceiveBeginPlay`
  (bind (_startlocation_x _startlocation_y _startlocation_z) (`KismetMathLibrary.BreakVector` (`self.StartLocation`)))
  (set `self.StartLocation` (`self.K2_GetActorLocation`))
  (bind _returnvalue (`GameplayStatics.GetActorOfClass` "/Game/FinalProject/Blueprints/BossPinto.BossPinto_C"))
  (bind (_direction _newtrack_0) (`Timeline|Glide` :!via `PlayFromStart`)
    (:`Update`
      (`self.K2_SetActorLocation` (`KismetMathLibrary.MakeVector` (`KismetMathLibrary.Lerp` _startlocation_x (- _startlocation_x 12000.0) _newtrack_0) _startlocation_y _startlocation_z)))
    (:`Finished`
      (`GameplayStatics.SpawnEmitterAtLocation` "/Game/StarterContent/Particles/P_Explosion.P_Explosion" (0.0 0.0 0.0) (struct) (100.0 100.0 100.0))
      (`self.K2_DestroyActor` _returnvalue)
      (`self.K2_DestroyActor`)
      (`|SpawnActorFromClass` "/Game/FinalProject/OurContent/EnemyContent/Squirrel_Content/Blueprints/Acorn/BP_Winning_Acorn.BP_Winning_Acorn_C" (`KismetMathLibrary.MakeTransform` (`self.K2_GetActorLocation`)) "Undefined" "OverrideRootScale" null null))))

(fn `UserConstructionScript`)