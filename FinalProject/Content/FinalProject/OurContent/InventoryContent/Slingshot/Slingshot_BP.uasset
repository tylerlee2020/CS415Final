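; Slingshot_BP is a pickup actor that adds the slingshot's item info to the player's HUD inventory.
; On BeginPlay it creates a pickup text widget and binds to the player's PickupItem dispatcher.
; Trigger overlaps show or remove the prompt and track whether the player is in range.
; When the dispatcher fires in range with collision enabled, it adds the item, hides and disables the actor, and refreshes the inventory.
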(event `self.ReceiveBeginPlay`
  (bind _iteminfo (`self.ItemInfo`))
  (bind _pickuptextreference (`self.PickupTextReference`))
  (bind (_item _itemimage _pickuptext) (break `/Game/FinalProject/OurContent/InventoryContent/InventoryStructure` _iteminfo))
  ;[1 1 1] Event BeginPlay
  (bind _returnvalue (`|CreateWidget` "/Game/FinalProject/OurContent/InventoryContent/PickupText_Widget.PickupText_Widget_C"))
  (set `self.PickupTextReference` _returnvalue)
  (setmembers `/Game/FinalProject/OurContent/InventoryContent/InventoryStructure` :`StructRef` _iteminfo :`Item` self) ; Select which item specificlly we are assigning
  (set `/Game/FinalProject/OurContent/InventoryContent/PickupText_Widget.PickupActor` _item _pickuptextreference)
  (set `/Game/FinalProject/OurContent/InventoryContent/PickupText_Widget.PickupText` _pickuptext _pickuptextreference)
  (bind _aszachs_first_person_character (cast `/Game/FinalProject/Blueprints/ZachsFirstPersonCharacter` (`GameplayStatics.GetPlayerCharacter` 0)))
  (bind _output_get (set `self.PlayerReference` _aszachs_first_person_character))
  (add `/Game/FinalProject/Blueprints/ZachsFirstPersonCharacter.PickupItem` _output_get (delegate `PickupItem_Event_0`)))

(event `PickupItem_Event_0`
  (bind _hud_widget (`/Game/FinalProject/Blueprints/ZachsFirstPersonCharacter.HUD_Widget` (`self.PlayerReference`)))
  ;[1 1 1] Pickup and add item to inventory, then refresh inventory
  (if (and (`self.GetActorEnableCollision`) (`self.WithinRangeOfItem`))
    (`KismetArrayLibrary.Array_Add` (`/Game/FinalProject/Widgets/HUD_Widget.Inventory` _hud_widget) (`self.ItemInfo`))
    (`Widget.RemoveFromParent` (`self.PickupTextReference`))
    (`self.SetActorHiddenInGame` true)
    (`self.SetActorEnableCollision` false)
    (`/Game/FinalProject/Widgets/HUD_Widget.Refresh Inventory` _hud_widget)))

(event `self.Trigger.OnComponentBeginOverlap`
  (params (OverlappedComponent :type "PrimitiveComponent Object Reference") (OtherActor :type "Actor Object Reference") (OtherComp :type "PrimitiveComponent Object Reference") (OtherBodyIndex :type Integer) (bFromSweep :type Boolean) (SweepResult :type "HitResult Structure (by ref)"))
  ;[1 1 1] Player within range?
  (cast `/Game/FinalProject/Blueprints/ZachsFirstPersonCharacter` OtherActor)
  (`UserWidget.AddToViewport` (`self.PickupTextReference`) 0)
  (set `self.WithinRangeOfItem` true))

(event `self.Trigger.OnComponentEndOverlap`
  (params (OverlappedComponent :type "PrimitiveComponent Object Reference") (OtherActor :type "Actor Object Reference") (OtherComp :type "PrimitiveComponent Object Reference") (OtherBodyIndex :type Integer))
  ;[1 1 1] Player within range?
  (cast `/Game/FinalProject/Blueprints/ZachsFirstPersonCharacter` OtherActor)
  (`Widget.RemoveFromParent` (`self.PickupTextReference`))
  (set `self.WithinRangeOfItem` false))

(fn `Pick Up Item`
  (returns (ItemToPickUp :type "Actor Object Reference"))
  (return null))

(fn `UserConstructionScript`)