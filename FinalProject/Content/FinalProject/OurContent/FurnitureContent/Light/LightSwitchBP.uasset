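; Wall light switch actor that toggles linked lights when the player presses E inside its trigger box.
; BeginPlay caches every LightBP in the level.
; Box overlap enables input and opens a Gate, and ending overlap reverses both.
; Each press messages lights sharing the switch's LightIndex and flips the switch mesh's tilt inside that loop, once per matching light.
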(event `self.ReceiveBeginPlay`
  (bind _outactors (`GameplayStatics.GetAllActorsOfClass` "/Game/FinalProject/OurContent/FurnitureContent/Light/LightBP.LightBP_C"))
  (for _array_element _outactors
    (`KismetArrayLibrary.Array_Add` (`self.LightArray`) _array_element)))

(event `self.Box.OnComponentBeginOverlap`
  (params (OverlappedComponent :type "PrimitiveComponent Object Reference") (OtherActor :type "Actor Object Reference") (OtherComp :type "PrimitiveComponent Object Reference") (OtherBodyIndex :type Integer) (bFromSweep :type Boolean) (SweepResult :type "HitResult Structure (by ref)"))
  (bind _switch_001_lightswitch_0 (`self.Switch_001_lightswitch_0`))
  (bind (_relativerotation_roll _relativerotation_pitch) (`KismetMathLibrary.BreakRotator` (`SceneComponent.RelativeRotation` (`self.Switch_001_lightswitch_0`))))
  (`self.EnableInput` (`GameplayStatics.GetPlayerController` 0))
  (goto _label :!via `Open`))

(event `self.Box.OnComponentEndOverlap`
  (params (OverlappedComponent :type "PrimitiveComponent Object Reference") (OtherActor :type "Actor Object Reference") (OtherComp :type "PrimitiveComponent Object Reference") (OtherBodyIndex :type Integer))
  (bind _switch_001_lightswitch_0 (`self.Switch_001_lightswitch_0`))
  (bind (_relativerotation_roll _relativerotation_pitch) (`KismetMathLibrary.BreakRotator` (`SceneComponent.RelativeRotation` (`self.Switch_001_lightswitch_0`))))
  (`self.DisableInput` (`GameplayStatics.GetPlayerController` 0))
  (goto _label :!via `Close`))

(event `Key|E`
  (params (Key :type "Key Structure"))
  (bind _switch_001_lightswitch_0 (`self.Switch_001_lightswitch_0`))
  (bind (_relativerotation_roll _relativerotation_pitch) (`KismetMathLibrary.BreakRotator` (`SceneComponent.RelativeRotation` (`self.Switch_001_lightswitch_0`))))
  (:`Pressed`
    (`/Engine/EditorBlueprintResources/StandardMacros.Gate` true :!label _label
      (:`Exit`
        (for _array_element (`self.LightArray`)
          (if (== (`/Game/FinalProject/OurContent/FurnitureContent/Light/LightBP.Light Index` _array_element) (`self.LightIndex`))
            (message `/Game/FinalProject/OurContent/FurnitureContent/Light/Lights_Int.Toggle Lights` _array_element)
            (if (== _relativerotation_pitch 0.0)
              (`SceneComponent.K2_SetRelativeRotation` _switch_001_lightswitch_0 (struct :`Pitch` -10.0) false false)
              (else
                (`SceneComponent.K2_SetRelativeRotation` :`self` _switch_001_lightswitch_0)))))))))

(fn `UserConstructionScript`)