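; BP_Keycard_Door is a keycard-locked door that swings open when given a matching DoorID.
; Its trigger box tracks whether ZachsFirstPersonCharacter is in range and, until the door is unlocked, shows the player's inventory and mouse cursor on entry.
; OpenDoor checks the ID, marks the door Complete and fires DoorOpen, where a timeline scales DoorAngle to rotate the mesh's yaw.
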(event `self.Box.OnComponentBeginOverlap`
  (params (OverlappedComponent :type "PrimitiveComponent Object Reference") (OtherActor :type "Actor Object Reference") (OtherComp :type "PrimitiveComponent Object Reference") (OtherBodyIndex :type Integer) (bFromSweep :type Boolean) (SweepResult :type "HitResult Structure (by ref)"))
  (bind _aszachs_first_person_character (cast `/Game/FinalProject/Blueprints/ZachsFirstPersonCharacter` OtherActor))
  (set `self.PlayerWithinRangeOfDoor` true)
  (if (not (`self.Complete`))
    (set `/Game/FinalProject/Widgets/HUD_Widget.InventoryVisible` "Visible" (`/Game/FinalProject/Blueprints/ZachsFirstPersonCharacter.HUD_Widget` _aszachs_first_person_character))
    (`/Game/FinalProject/Blueprints/ZachsFirstPersonCharacter.EnableMouseCursor` _aszachs_first_person_character)))

(event `self.Box.OnComponentEndOverlap`
  (params (OverlappedComponent :type "PrimitiveComponent Object Reference") (OtherActor :type "Actor Object Reference") (OtherComp :type "PrimitiveComponent Object Reference") (OtherBodyIndex :type Integer))
  (cast `/Game/FinalProject/Blueprints/ZachsFirstPersonCharacter` OtherActor)
  (set `self.PlayerWithinRangeOfDoor` false))

(event `DoorOpen`
  (bind (_direction _offsetval) (`Timeline|Timeline` :!via `PlayFromStart`)
    (:`Update`
      (`SceneComponent.K2_SetRelativeRotation` (`self.DoorMesh`) (`KismetMathLibrary.MakeRotator` 0.0 0.0 (* _offsetval (`self.DoorAngle`))) false false))))

(fn `openDoor`
  (params (Door_ID :type Integer))
  (if (== Door_ID (`self.Door_ID`))
    (set `self.Complete` true)
    (`self.DoorOpen`)
    (return)))

(fn `UserConstructionScript`)