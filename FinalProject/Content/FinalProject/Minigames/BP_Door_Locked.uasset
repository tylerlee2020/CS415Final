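; BP_Door_Locked is a keypad-locked minigame door that swings open once unlocked.
; Until it is complete, a ZachsFirstPersonCharacter entering its box pauses the game and gets a keypad widget with the mouse cursor shown.
; OpenDoor checks a door ID, marks the door complete and fires DoorOpen, whose timeline rotates the mesh's yaw toward DoorAngle.
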(event `self.Box.OnComponentBeginOverlap`
  (params (OverlappedComponent :type "PrimitiveComponent Object Reference") (OtherActor :type "Actor Object Reference") (OtherComp :type "PrimitiveComponent Object Reference") (OtherBodyIndex :type Integer) (bFromSweep :type Boolean) (SweepResult :type "HitResult Structure (by ref)"))
  (cast `/Game/FinalProject/Blueprints/ZachsFirstPersonCharacter` OtherActor)
  (if (not (`self.Complete`))
    (`GameplayStatics.SetGamePaused` true)
    (bind _returnvalue (`|CreateWidget` "/Game/FinalProject/Minigames/KeypadWidget.KeypadWidget_C"))
    (`UserWidget.AddToViewport` _returnvalue 0)
    (set `PlayerController.bShowMouseCursor` true (`GameplayStatics.GetPlayerController` 0)) ; Make sure that the player can see the mouse so that they know what they're clicking.
  ))

(event `DoorOpen`
  (bind (_direction _offsetval) (`Timeline|Timeline` :!via `PlayFromStart`)
    (:`Update`
      (`SceneComponent.K2_SetRelativeRotation` (`self.DoorMesh`) (`KismetMathLibrary.MakeRotator` 0.0 0.0 (* _offsetval (`self.DoorAngle`))) false false))))

(fn `openDoor`
  (params (Door_ID :type Integer))
  (if (== Door_ID (`self.Door_ID`))
    (set `self.Complete` true)
    (`self.DoorOpen`)
    (return)))

(fn `UserConstructionScript`)