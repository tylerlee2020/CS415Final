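; BP_Temp3 is a trigger actor that launches the connect-wire minigame when the player walks into its box.
; On overlap by ZachsFirstPersonCharacter, it pauses the game, creates the WWireBoard widget at a fixed viewport size and position, and shows the mouse cursor.
; If its Complete flag is already set, it only prints a debug string; this graph never sets that flag or unpauses the game.
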(event `self.ReceiveBeginPlay`)

(event `self.ReceiveActorBeginOverlap`
  (params (OtherActor :type "Actor Object Reference")))

(event `self.Box.OnComponentBeginOverlap`
  (params (OverlappedComponent :type "PrimitiveComponent Object Reference") (OtherActor :type "Actor Object Reference") (OtherComp :type "PrimitiveComponent Object Reference") (OtherBodyIndex :type Integer) (bFromSweep :type Boolean) (SweepResult :type "HitResult Structure (by ref)"))
  (cast `/Game/FinalProject/Blueprints/ZachsFirstPersonCharacter` OtherActor)
  (if (`self.Complete`)
    (`KismetSystemLibrary.PrintString` "hi there")
    (else
      (`GameplayStatics.SetGamePaused` true)
      (bind _returnvalue (`|CreateWidget` "/Game/FinalProject/Minigames/ConnectWire/wWireBoard.wWireBoard_C"))
      (`UserWidget.AddToViewport` _returnvalue 0)
      (`UserWidget.SetDesiredSizeInViewport` _returnvalue (1024.0 768.0))
      (`UserWidget.SetPositionInViewport` _returnvalue (420.0 75.0) true)
      (set `PlayerController.bShowMouseCursor` true (`GameplayStatics.GetPlayerController` 0)) ; Make sure that the player can see the mouse so that they know what they're clicking.
    )))

(fn `UserConstructionScript`)