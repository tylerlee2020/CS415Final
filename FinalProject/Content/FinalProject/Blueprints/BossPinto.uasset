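; BossPinto is an AI boss that spawns acorns and hurts the player on contact.
; A looping timer spawns BP_Acorn at SpawnAcorn, using an interval randomized once at BeginPlay.
; Pawn sensing sets the blackboard's HasSeenPlayer flag, cleared by a retriggerable delay after the last sighting.
; Capsule overlap launches the player along the boss's forward vector, reduces health, shows HurtWidget and shakes the camera.
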(event `self.ReceiveBeginPlay`
  ;[1 1 1] Fire acorn at player
  (`KismetSystemLibrary.K2_SetTimerDelegate` (delegate `BeginFire`) (`KismetMathLibrary.RandomFloatInRange` 1.0 10.0) true) ; Fire acorn with random time interval in between shots (takes between 1 and 10 seconds to fire another acorn)
)

(event `BeginFire`
  ;[1 1 1] Fire acorn at player
  (`|SpawnActorFromClass` "/Game/FinalProject/OurContent/EnemyContent/Squirrel_Content/Blueprints/Acorn/BP_Acorn.BP_Acorn_C" (`SceneComponent.K2_GetComponentToWorld` (`self.SpawnAcorn`)) "Undefined" "OverrideRootScale" null null))

(event `self.PawnSensing.OnSeePawn`
  (params (Pawn :type "Pawn Object Reference"))
  (bind _returnvalue (`AIBlueprintHelperLibrary.GetBlackboard` (`AIBlueprintHelperLibrary.GetAIController` self)))
  ;[1 1 1] When pawn is sensed run tree chase player part and then reset sense
  (cast `/Game/FinalProject/Blueprints/ZachsFirstPersonCharacter` Pawn)
  (`|ExecutionSequence`
    (:`then_0`
      (`BlackboardComponent.SetValueAsBool` _returnvalue "HasSeenPlayer" true))
    (:`then_1`
      (`KismetSystemLibrary.RetriggerableDelay` 5.0)
      (`BlackboardComponent.SetValueAsBool` _returnvalue "HasSeenPlayer" false))))

(event `self.Capsule.OnComponentBeginOverlap`
  (params (OverlappedComponent :type "PrimitiveComponent Object Reference") (OtherActor :type "Actor Object Reference") (OtherComp :type "PrimitiveComponent Object Reference") (OtherBodyIndex :type Integer) (bFromSweep :type Boolean) (SweepResult :type "HitResult Structure (by ref)"))
  ;[1 1 1] Camera Shake And Red Screen Effect Using BP_Shake And Hurt Widget Animation
  (bind _aszachs_first_person_character (cast `/Game/FinalProject/Blueprints/ZachsFirstPersonCharacter` OtherActor))
  (bind _returnvalue (`|CreateWidget` "/Game/FinalProject/Widgets/HurtWidget.HurtWidget_C"))
  (`UserWidget.AddToViewport` _returnvalue 0)
  (`self.LaunchCharacter` _aszachs_first_person_character (* (`self.GetActorForwardVector`) (`self.launch`)) false false)
  (set `/Game/FinalProject/Blueprints/ZachsFirstPersonCharacter.health` (`KismetMathLibrary.FClamp` (- (`/Game/FinalProject/Blueprints/ZachsFirstPersonCharacter.health` _aszachs_first_person_character) 10.0) 0.0 100.0) _aszachs_first_person_character)
  (`GameplayStatics.PlayWorldCameraShake` "/Game/FinalProject/Blueprints/BP_CamShake.BP_CamShake_C" (`self.K2_GetActorLocation` _aszachs_first_person_character) 0.0 100.0)
  (`KismetSystemLibrary.PrintString` "Hello"))

(fn `UserConstructionScript`)