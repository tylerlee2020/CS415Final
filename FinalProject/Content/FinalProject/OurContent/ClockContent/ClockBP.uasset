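; ClockBP is an analog clock that shows the current system time on rotating hour, minute and second hands.
; From BeginPlay, a one-second Delay loop reads Now and sets each hand's relative pitch as a negative angle.
; The hour hand adds a minute-based offset so it moves gradually between hours, while the minute and second hands step in whole units.
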(event `self.ReceiveBeginPlay`
  (bind (_year _month _day _hour _minute _second) (`KismetMathLibrary.BreakDateTime` (`KismetMathLibrary.Now`)))
  (`SceneComponent.K2_SetRelativeRotation` (`self.Hour Hand`) (`KismetMathLibrary.MakeRotator` 0.0 (* (+ (* (`KismetMathLibrary.Conv_IntToDouble` _hour) 30.0) (/ (`KismetMathLibrary.Conv_IntToDouble` _minute) 2.0)) -1.0)) false false :!label _label)
  (`SceneComponent.K2_SetRelativeRotation` (`self.Minutes Hand`) (`KismetMathLibrary.MakeRotator` 0.0 (* (`KismetMathLibrary.Conv_IntToDouble` _minute) -6.0)) false false)
  (`SceneComponent.K2_SetRelativeRotation` (`self.Clock_Seconds_Hand`) (`KismetMathLibrary.MakeRotator` 0.0 (* (`KismetMathLibrary.Conv_IntToDouble` _second) -6.0)) false false)
  (`KismetSystemLibrary.Delay` 1.0)
  (goto _label))

(fn `UserConstructionScript`)